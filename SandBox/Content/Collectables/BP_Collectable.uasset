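; BP_Collectable is a spinning pickup that counts down the Remaining total on BP_FirstPersonGameMode when collected.
; A fast looping timer calls Rotate to yaw the root component continuously.
; Any overlap with its Box plays a sound, decrements Remaining, shows a new WB_CollectWidget and destroys the actor.
; The overlapping actor is not filtered, as the character cast is left unconnected.
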(event `self.ReceiveBeginPlay`
  (`KismetSystemLibrary.K2_SetTimer` null "Rotate" 0.005 true))

(event `self.Box.OnComponentBeginOverlap`
  (params (OverlappedComponent :type "PrimitiveComponent Object Reference") (OtherActor :type "Actor Object Reference") (OtherComp :type "PrimitiveComponent Object Reference") (OtherBodyIndex :type Integer) (bFromSweep :type Boolean) (SweepResult :type "HitResult Structure (by ref)"))
  (`GameplayStatics.PlaySound2D` "/Game/SFX/little_robot_sound_factory_fantasy_Inventory_Open_01.little_robot_sound_factory_fantasy_Inventory_Open_01" 1.0 1.0 0.0 null null)
  (bind _asbp_first_person_game_mode (cast `/Game/GameModes/FirstPerson/Blueprints/BP_FirstPersonGameMode` (`GameplayStatics.GetGameMode`)))
  (bind _result (`/Engine/EditorBlueprintResources/StandardMacros.DecrementInt` (`/Game/GameModes/FirstPerson/Blueprints/BP_FirstPersonGameMode.Remaining` _asbp_first_person_game_mode))
    (:`  `
      (set `/Game/GameModes/FirstPerson/Blueprints/BP_FirstPersonGameMode.Remaining` _result _asbp_first_person_game_mode)
      (bind _returnvalue (`|CreateWidget` "/Game/Collectables/WB_CollectWidget.WB_CollectWidget_C"))
      (`UserWidget.AddToViewport` _returnvalue 0)
      (`self.K2_DestroyActor`))))

(fn `Rotate`
  (`SceneComponent.K2_AddLocalRotation` (`self.DefaultSceneRoot`) (`KismetMathLibrary.MakeRotator` 0.0 0.0 0.5) false false))

(fn `UserConstructionScript`)